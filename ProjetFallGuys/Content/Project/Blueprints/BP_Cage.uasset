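; BP_Cage is a team's goal cage that scores through BP_MainGameState when a BP_Ball enters it.
; On mesh overlap it fires a Niagara effect, deducts two points from its team, then gives all three teams one point.
; The team in slot 2 of the ball's last-touched array gets another point, then the ball is destroyed.
; A disconnected alternative scoring chain with ball respawning never runs.
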(event `self.ReceiveBeginPlay`
  (bind _asbp_main_game_state (cast `/Game/Project/Blueprints/BP_MainGameState` (`GameplayStatics.GetGameState`)))
  (set `self.MainGameState` _asbp_main_game_state))

(event `self.StaticMesh1.OnComponentBeginOverlap`
  (params (OverlappedComponent :type "PrimitiveComponent Object Reference") (OtherActor :type "Actor Object Reference") (OtherComp :type "PrimitiveComponent Object Reference") (OtherBodyIndex :type Integer) (bFromSweep :type Boolean) (SweepResult :type "HitResult Structure (by ref)"))
  (bind _asbp_ball (cast `/Game/Project/Blueprints/BP_Ball` OtherActor))
  (`ActorComponent.Activate` (`self.Niagara`) true)
  (`/Game/Project/Blueprints/BP_MainGameState.AddPoints` (`self.MainGameState`) (`self.indexTeam`) -2)
  (for _index (range 3)
    (`/Game/Project/Blueprints/BP_MainGameState.AddPoints` (`self.MainGameState`) _index 1))
  (`/Game/Project/Blueprints/BP_MainGameState.AddPoints` (`self.MainGameState`) (`|GetArrayItem` (`/Game/Project/Blueprints/BP_Ball.indexPlayerLastTouched` _asbp_ball) 2) 1)
  (`self.K2_DestroyActor` _asbp_ball))

(fn `UserConstructionScript`)