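; BP_Ball is a ball actor that records which player touched it last.
; When its static mesh is hit, it reads ListPlayer from BP_GameModeBase and, only if that list holds exactly three players, searches it for the hitting actor.
; A match stores that player's array index in IndexPlayerLastTouched.
; Tick and the construction script are empty, and a debug print of the index is left disconnected.
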(event `self.ReceiveTick`
  (params (DeltaSeconds :type "Float (single-precision)")))

(event `self.StaticMeshComponent.OnComponentHit`
  (params (HitComponent :type "PrimitiveComponent Object Reference") (OtherActor :type "Actor Object Reference") (OtherComp :type "PrimitiveComponent Object Reference") (NormalImpulse :type "Vector Structure") (Hit :type "HitResult Structure (by ref)"))
  (bind _returnvalue (`GameplayStatics.GetGameMode`))
  (bind _listplayer (`/Game/Project/Blueprints/BP_GameModeBase.listPlayer` (cast `/Game/Project/Blueprints/BP_GameModeBase` _returnvalue :!pure true)))
  (`/Engine/EditorBlueprintResources/StandardMacros.IsValid` _returnvalue
    (:`Is Valid`
      (if (== (`KismetArrayLibrary.Array_Length` _listplayer) 3)
        (for (_array_element _array_index) _listplayer
          (if (== OtherActor _array_element)
            (set `self.indexPlayerLastTouched` _array_index)))))))

(fn `UserConstructionScript`)