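; Lobby game instance that handles multiplayer session hosting, searching and joining.
; CreateSessionLobby creates a session and opens the given level as a listen server, while joining takes either a supplied search result or the first one found.
; Successful hosting or joining clears OnLobby, and outcomes are printed as debug strings.
; GetListRoom runs an online search without using its results, and GetListInfoRoom returns the stored NumberPlayers and NameServer variables.
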(event `JoinSessionLobby`
  (params (PlayerController :type "PlayerController Object Reference") (MaxResults :type Integer) (bUseLAN :type Boolean))
  (bind _results (`FindSessionsCallbackProxy.FindSessions` PlayerController MaxResults bUseLAN)
    (:`OnSuccess`
      (`JoinSessionCallbackProxy.JoinSession` PlayerController (`|GetArrayItem` _results)
        (:`OnSuccess`
          (`KismetSystemLibrary.PrintString` "Session has been joined")
          (set `self.OnLobby` false))
        (:`OnFailure`
          (`KismetSystemLibrary.PrintString` "Session join Failed"))))
    (:`OnFailure`
      (`KismetSystemLibrary.PrintString` "LAN Session Find Failed"))))

(event `JoinSpecificSession`
  (params (PlayerController :type "PlayerController Object Reference") (SearchResult :type "BlueprintSessionResult Structure (by ref)"))
  (`JoinSessionCallbackProxy.JoinSession` PlayerController SearchResult
    (:`OnSuccess`
      (`KismetSystemLibrary.PrintString` "Session has been joined")
      (set `self.OnLobby` false))
    (:`OnFailure`
      (`KismetSystemLibrary.PrintString` "Session join Failed"))))

(event `CreateSessionLobby`
  (params (PlayerController :type "PlayerController Object Reference") (PublicConnections :type Integer) (bUseLAN :type Boolean) (LevelName :type Name))
  (`CreateSessionCallbackProxy.CreateSession` PlayerController PublicConnections bUseLAN
    (:`OnSuccess`
      (`KismetSystemLibrary.PrintString` "Online Session Create")
      (set `self.OnLobby` false)
      (`GameplayStatics.OpenLevel` LevelName true "listen"))
    (:`OnFailure`
      (`KismetSystemLibrary.PrintString` "Online Session failed"))))

(event `GetListRoom`
  (`FindSessionsCallbackProxy.FindSessions` null 15))

(fn `GetListInfoRoom`
  (returns (NumberPlayers :type Integer) (NameServer :type Name))
  (return (`self.NumberPlayers`) (`self.NameServer`)))