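; Main HUD that puts the widget for the current minigame on screen once play leaves the lobby.
; BeginPlay caches BP_LobbyGameInstance, and Tick polls its lobby and level-load flags.
; When both are false, it swaps all widgets for the Football or Dash UI by EMiniGame, guarded by DoOnce, and marks the level loaded.
; A disconnected lobby-widget setup remains in the graph and never runs.
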(event `self.ReceiveBeginPlay`
  (set `self.LobbyGameInstance` (cast `/Game/Project/Blueprints/BP_LobbyGameInstance` (`GameplayStatics.GetGameInstance`) :!pure true)))

(event `self.ReceiveTick`
  (params (DeltaSeconds :type "Float (single-precision)"))
  (bind _lobbygameinstance (`self.LobbyGameInstance`))
  (if (`/Game/Project/Blueprints/BP_LobbyGameInstance.OnLobby` _lobbygameinstance)
    _
    (elif (`/Game/Project/Blueprints/BP_LobbyGameInstance.LevelIsLoad` _lobbygameinstance)
      _
      (elif (not (`self.DoOnce`))
        (switch `/Game/Project/Blueprints/MiniGame` (`/Game/Project/Blueprints/BP_LobbyGameInstance.EMiniGame` (`self.LobbyGameInstance`))
          (:`NewEnumerator0`
            (`WidgetLayoutLibrary.RemoveAllWidgets`)
            (bind _returnvalue (`|CreateWidget` "/Game/Project/Blueprints/Widget_UI.Widget_UI_C"))
            (`UserWidget.AddToViewport` _returnvalue 0)
            (`KismetSystemLibrary.PrintString` "Football Game")
            (set `self.DoOnce` true))
          (:`NewEnumerator1`
            (`WidgetLayoutLibrary.RemoveAllWidgets`)
            (bind _returnvalue_2 (`|CreateWidget` "/Game/Project/Blueprints/UI/Widget_Dash.Widget_Dash_C"))
            (`UserWidget.AddToViewport` _returnvalue_2 0)
            (`KismetSystemLibrary.PrintString` "Dash Game")
            (set `self.DoOnce` true)))
        (set `/Game/Project/Blueprints/BP_LobbyGameInstance.LevelIsLoad` true (`self.LobbyGameInstance`))))))

(fn `UserConstructionScript`)