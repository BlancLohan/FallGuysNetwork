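; DestroyableMap is a Blueprint for a map made of static mesh pieces that fall away over time.
; BeginPlay gathers eight mesh components into an ordered Parts array.
; Tick accumulates delta time and, each time FallingInterval elapses, enables physics simulation on the next part and resets the timer.
; The sequence stops after six parts, leaving the last two without physics enabled by this graph.
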(event `self.ReceiveBeginPlay`
  (set `self.TimeStocker` 0.0)
  (set `self.Parts` (`|MakeArray` (`self.StaticMesh`) (`self.StaticMesh1`) (`self.StaticMesh2`) (`self.StaticMesh3`) (`self.StaticMesh4`) (`self.StaticMesh5`) (`self.StaticMesh6`) (`self.StaticMesh7`))))

(event `self.ReceiveTick`
  (params (DeltaSeconds :type "Float (single-precision)"))
  (bind _output_get (set `self.TimeStocker` (+ DeltaSeconds (`self.TimeStocker`))))
  (if (and (>= _output_get (`self.FallingInterval`)) (< (`self.NbrFallenParts`) 6))
    (`PrimitiveComponent.SetSimulatePhysics` (`|GetArrayItem` (`self.Parts`) (`self.NbrFallenParts`)) true)
    (set `self.NbrFallenParts` (+ (`self.NbrFallenParts`) 1))
    (set `self.TimeStocker` 0.0)))

(fn `UserConstructionScript`)