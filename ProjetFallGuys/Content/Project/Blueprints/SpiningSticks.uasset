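; SpiningSticks is a rotating obstacle that knocks third-person characters back on contact.
; Once the game state reports the game has started, Tick plays an acceleration timeline whose curve scales the yaw rotation of the lower and middle cylinders, each with its own speed multiplier.
; On a hit, it launches the character away from the struck component's origin, adding to their current velocity.
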(event `self.ReceiveBeginPlay`
  (set `self.maingamestate` (cast `/Game/Project/Blueprints/BP_MainGameState` (`GameplayStatics.GetGameState`) :!pure true)))

(event `self.ReceiveTick`
  (params (DeltaSeconds :type "Float (single-precision)"))
  (if (`/Game/Project/Blueprints/BP_MainGameState.isGameStarted?` (`self.maingamestate`))
    (bind (_direction _newtrack_0) (`Timeline|TimeLineAcceleration`)
      (:`Update`
        (`|ExecutionSequence`
          (:`then_0`
            (`SceneComponent.K2_AddWorldRotation` (`self.ParentCylinderDown`) (`KismetMathLibrary.MakeRotator` 0.0 0.0 (* (`self.SpeedMultiplierDown`) _newtrack_0)) false false))
          (:`then_1`
            (`SceneComponent.K2_AddWorldRotation` (`self.ParentCylinderMiddle`) (`KismetMathLibrary.MakeRotator` 0.0 0.0 (* (`self.SpeedMultiplierMiddle`) _newtrack_0)) false false)))))))

(event `self.ReceiveHit`
  (params (MyComp :type "PrimitiveComponent Object Reference") (Other :type "Actor Object Reference") (OtherComp :type "PrimitiveComponent Object Reference") (bSelfMoved :type Boolean) (HitLocation :type "Vector Structure") (HitNormal :type "Vector Structure") (NormalImpulse :type "Vector Structure") (Hit :type "HitResult Structure (by ref)"))
  (bind _asthird_person_character (cast `/Game/ThirdPersonCPP/Blueprints/ThirdPersonCharacter` Other))
  (`Character.LaunchCharacter` _asthird_person_character (* (`KismetMathLibrary.GetDirectionUnitVector` HitLocation (`SceneComponent.K2_GetComponentLocation` MyComp)) -200) false false))

(fn `UserConstructionScript`)