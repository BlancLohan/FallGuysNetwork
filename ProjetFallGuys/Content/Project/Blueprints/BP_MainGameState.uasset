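; Game state for team minigames that tracks three team scores, a round timer and the win condition.
; Tick flags a win by score in Football or last player standing in Dash and Fallcase, based on the game instance's mode.
; Tick also resets UI countdowns on request, or spawns the ball on authority once a countdown finishes and none exists.
; ManageTimer flags a reset at zero, and a RepNotify restores points and timer.
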(event `resetUI`
  (bind _foundwidgets (`WidgetBlueprintLibrary.GetAllWidgetsOfClass` "/Game/Project/Blueprints/Widget_UI.Widget_UI_C"))
  (for _array_element _foundwidgets
    (set `/Game/Project/Blueprints/Widget_UI.timerCountdown` 4.0 _array_element)
    (`Widget.SetVisibility` (`/Game/Project/Blueprints/Widget_UI.TxtCountdown` _array_element) "Visible"))
  (set `self.needResetCountdown` false))

(event `self.ReceiveBeginPlay`
  (set `self.Timer` (`self.TimeMaxRound`)))

(event `self.ReceiveTick`
  (params (DeltaSeconds :type "Float (single-precision)"))
  (`self.WinCondition`)
  (if (`self.needResetCountdown`)
    (`self.resetUI`)
    (else
      (bind _foundwidgets (`WidgetBlueprintLibrary.GetAllWidgetsOfClass` "/Game/Project/Blueprints/Widget_UI.Widget_UI_C"))
      (for _array_element _foundwidgets
        (if (`/Game/Project/Blueprints/Widget_UI.isCountdownFinished?` _array_element)
          (`/Engine/EditorBlueprintResources/ActorMacros.Switch Has Authority`
            (:`Authority`
              (bind _outactors (`GameplayStatics.GetAllActorsOfClass` "/Game/Project/Blueprints/BP_Ball.BP_Ball_C"))
              (if (== (`KismetArrayLibrary.Array_Length` _outactors) 0)
                (`|SpawnActorFromClass` "/Game/Project/Blueprints/BP_Ball.BP_Ball_C" (`KismetMathLibrary.MakeTransform` (10.0 -930.0 500.0)) "Undefined" "OverrideRootScale" null null)
                (set `/Game/Project/Blueprints/Widget_UI.isCountdownFinished?` false _array_element)
                (`KismetSystemLibrary.PrintString` "Hello")))))))))

(fn `AddPoints`
  (params (Team :type Integer) (pointToAdd :type Integer))
  (switch `int` Team
    (:`0`
      (set `self.PointTeam1` (+ (`self.PointTeam1`) pointToAdd)))
    (:`1`
      (set `self.PointTeam2` (+ (`self.PointTeam2`) pointToAdd)))
    (:`2`
      (set `self.PointTeam3` (+ (`self.PointTeam3`) pointToAdd)))))

(fn `ManageTimer`
  (params (DeltaTime :type "Float (double-precision)"))
  (if (> (`self.Timer`) 0.0)
    (set `self.Timer` (- (`self.Timer`) DeltaTime))
    (else
      (set `self.Timer` 0.0)
      (set `self.ResetTimerAndPoints` true))))

(fn `OnRep_ResetPoints`
  (set `self.PointTeam1` 0)
  (set `self.PointTeam2` 0)
  (set `self.PointTeam3` 0)
  (set `self.Timer` (`self.TimeMaxRound`)))

(fn `UserConstructionScript`)

(fn `WinCondition`
  (locals (playerAlive :type Integer))
  (bind _pointsforwin (`self.pointsForWin`))
  (if (`self.isGameStarted?`)
    (switch `/Game/Project/Blueprints/MiniGame` (`/Game/Project/Blueprints/BP_LobbyGameInstance.EMiniGame` (cast `/Game/Project/Blueprints/BP_LobbyGameInstance` (`GameplayStatics.GetGameInstance`) :!pure true))
      (:`NewEnumerator0`
        (if (or (>= (`self.PointTeam1`) _pointsforwin) (>= (`self.PointTeam2`) _pointsforwin) (>= (`self.PointTeam3`) _pointsforwin))
          (set `self.teamHaveWin?` true)))
      (:`NewEnumerator1`
        (bind _outactors (`GameplayStatics.GetAllActorsOfClass` "/Game/ThirdPersonCPP/Blueprints/ThirdPersonCharacter.ThirdPersonCharacter_C" :!label _label))
        (for _array_element _outactors
          (if (not (`/Game/ThirdPersonCPP/Blueprints/ThirdPersonCharacter.deafeat?` _array_element))
            (`/Engine/EditorBlueprintResources/StandardMacros.IncrementInt` (`local.playerAlive`))))
        (if (== (`local.playerAlive`) 1)
          (set `self.teamHaveWin?` true)))
      (:`NewEnumerator2`
        (goto _label)))))