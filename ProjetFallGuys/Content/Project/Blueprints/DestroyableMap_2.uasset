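; Destroyable map actor that drops its static mesh pieces one at a time during a match, shrinking the level.
; On server Tick, once BP_MainGameState reports the game started, a timer picks and removes a random piece from Parts every FallingInterval until two remain.
; The current piece warns by alternating random jitter with position restores, then sinks a fixed step per tick, so fall speed is frame-rate dependent.
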(event `self.ReceiveBeginPlay`
  (set `self.TimeStocker` 0.0)
  (set `self.Parts` (`|MakeArray` (`self.StaticMesh9`) (`self.StaticMesh6`) (`self.StaticMesh7`) (`self.StaticMesh8`) (`self.StaticMesh5`) (`self.StaticMesh10`) (`self.StaticMesh11`) (`self.StaticMesh12`) (`self.StaticMesh13`))))

(event `self.ReceiveTick`
  (params (DeltaSeconds :type "Float (single-precision)"))
  (bind (_positionstocker_x _positionstocker_y _positionstocker_z) (`KismetMathLibrary.BreakVector` (`self.PositionStocker`)))
  (bind _itemsotcker (`self.ItemSotcker`))
  (bind _itemsotcker_2 (`self.ItemSotcker`))
  (`/Engine/EditorBlueprintResources/ActorMacros.Switch Has Authority`
    (:`Authority`
      (if (`/Game/Project/Blueprints/BP_MainGameState.isGameStarted?` (cast `/Game/Project/Blueprints/BP_MainGameState` (`GameplayStatics.GetGameState`) :!pure true))
        (`|ExecutionSequence`
          (:`then_0`
            (if (`self.StartFalling`)
              (set `self.LastTremblingTime` (+ (`self.LastTremblingTime`) DeltaSeconds))
              (if (< (`self.TimeStocker`) 1.5)
                (if (> (`self.LastTremblingTime`) 0.1)
                  ;[1 1 1] Trembling
                  (if (`self.Trembled`)
                    (`SceneComponent.K2_SetWorldLocation` _itemsotcker_2 (`self.PositionStocker`) true false)
                    (set `self.Trembled` false)
                    (set `self.LastTremblingTime` 0.0)
                    (else
                      (bind _output_get (set `self.PositionStocker` (`SceneComponent.K2_GetComponentLocation` _itemsotcker_2)))
                      (`SceneComponent.K2_SetWorldLocation` _itemsotcker_2 (`KismetMathLibrary.MakeVector` (+ (.x _output_get) (* (`KismetMathLibrary.Conv_IntToDouble` (`KismetMathLibrary.RandomIntegerInRange` (`self.Min`) (`self.Max`))) 1.0)) (+ (.y _output_get) (* (`KismetMathLibrary.Conv_IntToDouble` (`KismetMathLibrary.RandomIntegerInRange` (`self.Min`) (`self.Max`))) 1.0)) (+ (.z _output_get) (* (`KismetMathLibrary.Conv_IntToDouble` (`KismetMathLibrary.RandomIntegerInRange` (`self.Min`) (`self.Max`))) 1.0))) true false)
                      (set `self.Trembled` true)
                      (set `self.LastTremblingTime` 0.0))))
                (else
                  ;[1 1 1] Falling
                  (if (`self.Trembled`)
                    (`SceneComponent.K2_SetWorldLocation` _itemsotcker (`self.PositionStocker`) false true)
                    (set `self.Trembled` false)
                    (else
                      (bind _output_get_2 (set `self.PositionStocker` (`KismetMathLibrary.MakeVector` _positionstocker_x _positionstocker_y (- _positionstocker_z 5.0))))
                      (`SceneComponent.K2_SetWorldLocation` _itemsotcker _output_get_2 false true)))))))
          (:`then_1`
            (bind _output_get_3 (set `self.TimeStocker` (+ DeltaSeconds (`self.TimeStocker`))))
            (if (and (>= _output_get_3 (`self.FallingInterval`)) (> (`KismetArrayLibrary.Array_LastIndex` (`self.Parts`)) 1))
              (bind _output_get_4 (set `self.RandomStocker` (`KismetMathLibrary.RandomIntegerInRange` 0 (`KismetArrayLibrary.Array_LastIndex` (`self.Parts`)))))
              (set `self.StartFalling` true)
              (set `self.ItemSotcker` (`|GetArrayItem` (`self.Parts`) _output_get_4))
              (`KismetArrayLibrary.Array_Remove` (`self.Parts`) _output_get_4)
              (set `self.TimeStocker` 0.0)
              (set `self.LastTremblingTime` 0.0))))))))

(fn `UserConstructionScript`)